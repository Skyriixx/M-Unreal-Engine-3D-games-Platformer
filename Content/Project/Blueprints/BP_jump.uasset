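; Character jump logic, bound to its owner, that adds variable-height jumping and timing aids.
; A Gravity event, not called here, applies vertical impulses scaled by rise, fall and whether jump is held.
; Movement-mode changes timestamp walking off ledges for coyote time, though nothing reads it, and re-jump on landing within the buffer window.
; Presses register only while Walking, so that buffer measures from the last grounded press.
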(event `self.ReceiveBeginPlay`
  ;[0.5468 0 1] Event binding
  (bind _ascharacter (cast `Character` (`self.GetOwner`)))
  (bind _output_get (set `self.Character` _ascharacter))
  (set `self.CharacterMovement` (`Character.CharacterMovement` _output_get))
  (add `Character.MovementModeChangedDelegate` _output_get (delegate `MovementModeChanged`)))

(event `InputAction|Jump` :consume false :overrideparent false
  (params (Key :type "Key Structure"))
  (bind _character (`self.Character`))
  ;[0 0.0615 1] Jump triggering
  (:`Pressed`
    (switch `EMovementMode` (`CharacterMovementComponent.MovementMode` (`self.CharacterMovement`))
      (:`MOVE_Walking`
        (set `self.JumpPressed` true)
        (set `self.Jumping` true)
        (set `self.JumpPressedTime` (`GameplayStatics.GetTimeSeconds`))
        (`Character.Jump` _character))))
  (:`Released`
    (set `self.JumpPressed` false)
    (`Character.StopJumping` _character)))

(event `InputVectorAxis|Gravity`
  (params (AxisValue :type "Vector Structure"))
  (bind (_returnvalue_x _returnvalue_y _returnvalue_z) (`KismetMathLibrary.BreakVector` (`Actor.GetVelocity` (`self.Character`))))
  ;[0 1 0.1891] Variable height jump
  (if (>= _returnvalue_z 0.0)
    ;;[1 0.3345 0.89] Rising
    (if (`self.JumpPressed`)
      (set `self.GravityScale` 1.0)
      (else
        (set `self.GravityScale` (- (`self.LowJumpGravityMultiplier`) 1.0))))
    (else
      ;;[1 0.3345 0.89] Falling
      (set `self.GravityScale` (- (`self.FallGravityMultiplier`) 1.0))))
  (`CharacterMovementComponent.AddImpulse` (`self.CharacterMovement`) (`KismetMathLibrary.MakeVector` 0.0 0.0 (* (`MovementComponent.GetGravityZ` (`self.CharacterMovement`)) (- (`self.GravityScale`) 1.0))) false))

(event `MovementModeChanged`
  (params (Character :type "Character Object Reference") (PrevMovementMode :type "EMovementMode Enum" :default "MOVE_None") (PreviousCustomMode :type Byte))
  (bind _movementmode (`CharacterMovementComponent.MovementMode` (`Character.CharacterMovement` Character)))
  (switch `EMovementMode` PrevMovementMode
    (:`MOVE_Walking`
      ;[0.9042 1 0] Coyote time
      (switch `EMovementMode` _movementmode
        (:`MOVE_Falling`
          (if (not (`self.Jumping`))
            (set `self.FloatingTime` (`GameplayStatics.GetTimeSeconds`))))))
    (:`MOVE_Falling`
      ;[0 1 0.9878] Jump buffering
      (switch `EMovementMode` _movementmode
        (:`MOVE_Walking`
          (if (<= (- (`GameplayStatics.GetTimeSeconds`) (`self.JumpPressedTime`)) (`self.JumpBufferTime`))
            (`Character.Jump` (`self.Character`))
            (else
              (set `self.Jumping` false))))))))