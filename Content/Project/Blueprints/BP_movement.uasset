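; BP_movement is a component that gives its owning Character movement and mouse-look style camera control from input axes.
; On BeginPlay it caches the owner's camera component and the owner cast to Character.
; Forward and Right axes add movement input along the camera's world forward and right vectors, scaled by Speed.
; LookRight and LookUp feed controller yaw and pitch, with pitch inverted.
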(event `self.ReceiveBeginPlay`
  (bind _returnvalue (`self.GetOwner`))
  ;[0.4388 0 1] Init
  (set `self.Camera` (`Actor.GetComponentByClass` _returnvalue "/Script/Engine.CameraComponent"))
  (bind _ascharacter (cast `Character` _returnvalue))
  (set `self.Character` _ascharacter))

(event `InputAxis|Forward`
  (params (AxisValue :type "Float (single-precision)"))
  ;[0.2183 0.1567 1] Movement
  ;;[1 1 1] Forward movement
  (`Pawn.AddMovementInput` (`self.Character`) (`KismetMathLibrary.GetForwardVector` (`SceneComponent.K2_GetComponentRotation` (`self.Camera`))) (* AxisValue (`self.Speed`)) false))

(event `InputAxis|Right`
  (params (AxisValue :type "Float (single-precision)"))
  ;[0.2183 0.1567 1] Movement
  ;;[1 1 1] Right movement
  (`Pawn.AddMovementInput` (`self.Character`) (`KismetMathLibrary.GetRightVector` (`SceneComponent.K2_GetComponentRotation` (`self.Camera`))) (* AxisValue (`self.Speed`)) false))

(event `InputAxis|LookRight`
  (params (AxisValue :type "Float (single-precision)"))
  ;[1 0 0.1624] Camera movement
  ;;[1 1 1] Look X axis
  (`Pawn.AddControllerYawInput` (`self.Character`) AxisValue))

(event `InputAxis|LookUp`
  (params (AxisValue :type "Float (single-precision)"))
  ;[1 0 0.1624] Camera movement
  ;;[1 1 1] Look Y axis
  (`Pawn.AddControllerPitchInput` (`self.Character`) (* AxisValue -1.0)))